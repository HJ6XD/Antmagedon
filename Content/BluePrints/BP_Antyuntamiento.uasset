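; BP_Antyuntamiento is a clickable structure actor with highlight effects and a function that spawns worker ants (BP_HormigaObrera).
; On BeginPlay, BPRuntimeMat applies a runtime material to Estructura and zeroes its FresnelMask and FlickerMask.
; Flicker and Fresnel events tween those parameters; clicking the structure fades the Fresnel off.
; SpawnAnt places a worker at SpawnTransform's location offset by the actor's location, using the actor's rotation and scale.
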(event OnClicked(Estructura)
  (params (TouchedComponent :type Primitive%20Component%20Object%20Reference) (ButtonPressed :type Key%20Structure :default "None"))
  (CallFunction|Fresnel false))

(event Custom|Flicker
  (|CollapseGraph_2_2_2))

(event Custom|Fresnel
  (params (SetActive :type Boolean))
  (|CollapseGraph_0_2_2_2 SetActive))

(event EventBeginPlay
  (|CollapseGraph_1_2_2_2))

(fn ConstructionScript)

(fn SpawnAnt
  (bind _returnvalue (Transformation|GetActorTransform))
  (Game|SpawnActorfromClass "/Game/BluePrints/BP_HormigaObrera.BP_HormigaObrera_C" (Math|Transform|MakeTransform (+ (.location (Variables|Default|GetSpawn%20Transform)) (.location _returnvalue)) (.rotation _returnvalue) (.scale _returnvalue)) "Undefined" "MultiplyWithRoot" 0 0))