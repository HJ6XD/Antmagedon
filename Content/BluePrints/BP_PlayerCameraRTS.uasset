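; RTS camera pawn that pans over the map and issues move orders to selected ant units.
; Enhanced Input moves it along X and Y at an altitude set on BeginPlay.
; The move action line-traces toward the mouse cursor, then GiveOrder sends the game manager's selection to the hit building or point, unless the last selected is a BP_HormigaGuerreraNegra.
; It also exposes a camera shake event.
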(event Custom|Give%20Order
  (bind _asbp_rtsgame_manager (Utilities|Casting|CastToBP_RTSGameManager (Game|GetGameMode)))
  (bind _asbp_hormiga_t (Utilities|Casting|CastToBP_HormigaT (Variables|/Game/BluePrints/BP_RTSGameManager.BP_RTSGameManager_C|GetLastSelected _asbp_rtsgame_manager)))
  (Utilities|Casting|CastToBP_HormigaGuerreraNegra _asbp_hormiga_t
    (:CastFailed
      (for _array_element (Variables|/Script/Antmagedon.RTSGameManager|GetselectedList _asbp_rtsgame_manager)
        (bind _asbp_hormiga_t_2 (Utilities|Casting|CastToBP_HormigaT _array_element))
        (bind _targetbuild (Variables|Default|GetTargetBuild)
          (:then
            (Default|MovetoActor _asbp_hormiga_t_2 _targetbuild))
          (:else
            (Default|MovetoPosition _asbp_hormiga_t_2 (Variables|Default|GetDestination)))))
      (Audio|PlaySound2D (Variables|Default|GetOrderSound) 1.0 1.0 0.0 0 0))))

(event Custom|ShakeCamera
  (params (ShakeScale :type Float%20%28double-precision%29))
  (if (<= ShakeScale 0.0)
    (Variables|Default|SettargetShakeScale ShakeScale)
    (else
      (Variables|Default|SettargetShakeScale 1.0)))
  (CameraShakes|StartCameraShake (Variables|/Script/Engine.PlayerController|GetPlayerCameraManager (Game|GetPlayerController 0)) "/Game/Camara/BP_RegularCameraShake.BP_RegularCameraShake_C" (Variables|Default|GettargetShakeScale) "CameraLocal" "0, 0, 0"))

(event Input|EnhancedActionEvents|EnhancedInputActionIA_VerticalMovement
  (params (ActionValue :type Float%20%28double-precision%29) (ElapsedSeconds :type Float%20%28double-precision%29) (TriggeredSeconds :type Float%20%28double-precision%29) (InputAction :type Input%20Action%20Object%20Reference :default "/Game/BluePrints/InputActions/IA_VerticalMovement.IA_VerticalMovement"))
  (bind _returnvalue (Transformation|GetActorLocation))
  (Transformation|SetActorLocation (Math|Vector|MakeVector (+ (* (* ActionValue (Variables|Default|GetMovementSpeed)) (Utilities|Time|GetWorldDeltaSeconds)) (.x _returnvalue)) (.y _returnvalue) (.z _returnvalue)) false false))

(event Input|EnhancedActionEvents|EnhancedInputActionIA_HorizontalMovement
  (params (ActionValue :type Float%20%28double-precision%29) (ElapsedSeconds :type Float%20%28double-precision%29) (TriggeredSeconds :type Float%20%28double-precision%29) (InputAction :type Input%20Action%20Object%20Reference :default "/Game/BluePrints/InputActions/IA_HorizontalMovement.IA_HorizontalMovement"))
  (bind _returnvalue (Transformation|GetActorLocation))
  (Transformation|SetActorLocation (Math|Vector|MakeVector (.x _returnvalue) (+ (* (* ActionValue (Variables|Default|GetMovementSpeed)) (Utilities|Time|GetWorldDeltaSeconds)) (.y _returnvalue)) (.z _returnvalue)) false false))

(event Input|EnhancedActionEvents|EnhancedInputActionIA_MoveTo
  (params (ActionValue :type Boolean) (ElapsedSeconds :type Float%20%28double-precision%29) (TriggeredSeconds :type Float%20%28double-precision%29) (InputAction :type Input%20Action%20Object%20Reference :default "/Game/BluePrints/InputActions/IA_MoveTo.IA_MoveTo"))
  (bind _camera (Variables|Default|GetCamera))
  (bind _returnvalue (Transformation|GetWorldLocation _camera))
  (Variables|Default|SetTargetBuild 0)
  (bind _outhit (Collision|LineTraceByChannel _returnvalue (* (- (.WorldLocation (Game|Player|ConvertMouseLocationToWorldSpace (Game|GetPlayerController 0))) _returnvalue) (Variables|Default|GetRange)) "TraceTypeQuery1" false 0 "ForDuration" true "(R=1.000000,G=0.000000,B=0.000000,A=1.000000)" "(R=0.000000,G=1.000000,B=0.000000,A=1.000000)" 0.0))
  (Variables|Default|SetDestination (.location _outhit))
  (Utilities|IsValid (.hitactor _outhit)
    (:Is%20Valid
      (bind _asbp_edificio (Utilities|Casting|CastToBP_Edificio (.hitactor _outhit))
        (:then
          (Variables|Default|SetTargetBuild _asbp_edificio))
        (:CastFailed
          _))
      (CallFunction|GiveOrder))))

(event EventBeginPlay
  (bind _returnvalue (Transformation|GetActorLocation))
  (Transformation|SetActorLocation (Math|Vector|MakeVector (.x _returnvalue) (.y _returnvalue) (Variables|Default|GetAlttitude)) false false)
  (Transformation|SetActorRotation (Math|Rotator|MakeRotator 0.0 (.pitch (Transformation|GetActorRotation)) 0.0)))

(fn ConstructionScript)