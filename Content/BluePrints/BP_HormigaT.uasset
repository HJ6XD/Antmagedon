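; BP_HormigaT is a selectable RTS ant unit that moves on command, takes damage and dies.
; Clicking its selection trigger toggles it in the BP_RTSGameManager selected list, and GiveAction sends it via AI MoveTo.
; A runtime material drives tweened Fresnel selection highlight, damage flicker and dither on death.
; Death occurs when HP drops below zero, setting the animation flag, playing a sound and removing it from selection.
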(event OnClicked(SelectionTrigger)
  (params (TouchedComponent :type Primitive%20Component%20Object%20Reference) (ButtonPressed :type Key%20Structure :default "None"))
  (CallFunction|ToggleSelect))

(event Custom|Flicker
  (|CollapsedFlicker))

(event Custom|Fresnel
  (params (SetActive :type Boolean))
  (|CollapsedFresnel SetActive))

(event Custom|OnAntDead
  (|CollapsedAntDeath))

(event Custom|ToggleSelect
  (|CollapsedToggleSelected))

(event Custom|Deselect
  (CallFunction|Fresnel false))

(event Custom|GiveAction
  (params (Target :type Vector))
  (AI|AIMoveTo self Target 0 5e+01 true
    (:OnSuccess
      (Development|PrintText "succsess" true true "(R=0.000000,G=1.000000,B=0.047969,A=1.000000)"))
    (:OnFail
      (Development|PrintText "fail" true true "(R=1.000000,G=0.043185,B=0.000000,A=1.000000)"))))

(event Custom|Dither
  (|CollapsedDither))

(event Custom|AntRecibeDamage
  (params (dmg :type Integer))
  (|CollapsedRecibeDamage dmg))

(event EventBeginPlay
  (|CollapsedBeginPlay))

(fn ConstructionScript)