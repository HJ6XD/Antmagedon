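; BP_Tile is a cube tile actor that fades a fresnel highlight in and out when the cursor hovers over it.
; On BeginPlay, its BPRuntimeMat component applies a runtime material to the cube.
; Cursor-over events call Fresnel, which tweens the material's fresnelMask scalar from its current value toward on or off over a short duration.
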(event OnBeginCursorOver(Cube)
  (params (TouchedComponent :type Primitive%20Component%20Object%20Reference))
  (CallFunction|Fresnel true))

(event OnEndCursorOver(Cube)
  (params (TouchedComponent :type Primitive%20Component%20Object%20Reference))
  (CallFunction|Fresnel false))

(event Custom|Fresnel
  (params (SetActive :type Boolean))
  (|FresnelCollapsed SetActive))

(event EventBeginPlay
  (Default|ApplyRuntimeMaterial (Variables|Default|GetBP_RuntimeMat) (Utilities|Array|MakeArray (Variables|Default|GetCube))))

(event Collision|EventActorBeginOverlap
  (params (OtherActor :type Actor%20Object%20Reference)))

(event EventTick
  (params (DeltaSeconds :type Float%20%28single-precision%29)))

(fn ConstructionScript)