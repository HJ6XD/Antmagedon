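; Black warrior ant unit that picks an enemy to attack, built on a parent Blueprint.
; BeginPlay sets its max and current HP, then calls RepeatingAction.
; RepeatingAction runs the parent logic, then scans OutActors for the first BP_Antyuntamiento or BP_HormigaT that is not another black warrior.
; That match becomes TargetActorToAtack and triggers Atack, with list order deciding priority.
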(event EventBeginPlay
  (|CallParentFunction)
  (bind _output_get (Variables|Default|SetmaxHP 120))
  (Variables|Default|SetcurHP _output_get)
  (CallFunction|RepeatingAction))

(event EventTick
  (params (DeltaSeconds :type Float%20%28single-precision%29))
  (|CallParentFunction DeltaSeconds) ; This node is disabled and will not be called.\nDrag off pins to build functionality.
)

(fn ConstructionScript
  (|CallParentFunction))

(fn RepeatingAction
  (|CallParentFunction)
  (for _array_element (Variables|Default|GetOut%20Actors)
    (bind _asbp_antyuntamiento (Utilities|Casting|CastToBP_Antyuntamiento _array_element)
      (:then
        (Variables|Default|SetTargetActorToAtack _asbp_antyuntamiento))
      (:CastFailed
        (bind _asbp_hormiga_t (Utilities|Casting|CastToBP_HormigaT _array_element))
        (Utilities|Casting|CastToBP_HormigaGuerreraNegra _asbp_hormiga_t
          (:CastFailed
            (Variables|Default|SetTargetActorToAtack _asbp_hormiga_t)))))
    (CallFunction|Atack)
    (return false))
  (return false))