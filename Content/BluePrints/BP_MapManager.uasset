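; BP_MapManager is an actor that builds a square grid of BP_Tile actors when play begins.
; CreateTileMap runs nested loops over WidthAndHeight, spawning each tile at a base transform, then teleporting it to an X/Y position spaced by Offset.
; Each tile is stored in TileMap, keyed by its computed world X/Y position rather than its grid index.
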(event Custom|CreateTileMap
  (for _index (range 0 (Variables|Default|GetWidthAndHeight))
    (for _index_2 (range 0 (Variables|Default|GetWidthAndHeight))
      (bind _returnvalue (Game|SpawnActorfromClass "/Game/BluePrints/BP_Tile.BP_Tile_C" (Variables|Default|GetBase%20Transform) "Undefined" "MultiplyWithRoot" 0 0))
      (Transformation|SetActorLocation _returnvalue (Math|Vector|MakeVector (Math|Conversions|ToFloat(Integer) (* _index (Variables|Default|GetOffset))) (Math|Conversions|ToFloat(Integer) (* _index_2 (Variables|Default|GetOffset))) 0.0) false true)
      (Utilities|Map|Add (Variables|Default|GetTileMap) (Math|Vector2D|MakeVector2D (Math|Conversions|ToFloat(Integer) (* _index (Variables|Default|GetOffset))) (Math|Conversions|ToFloat(Integer) (* _index_2 (Variables|Default|GetOffset)))) _returnvalue))))

(event EventBeginPlay
  (CallFunction|CreateTileMap))

(event Collision|EventActorBeginOverlap
  (params (OtherActor :type Actor%20Object%20Reference)))

(event EventTick
  (params (DeltaSeconds :type Float%20%28single-precision%29)))

(fn ConstructionScript)