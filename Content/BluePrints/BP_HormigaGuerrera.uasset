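; BP_HormigaGuerrera is a warrior ant with mouse-driven material feedback on its mesh.
; BPRuntimeMat applies a runtime material at BeginPlay, with fresnel and flicker masks starting at zero.
; Cursor-over tweens the fresnel in, with no cursor-exit handler to clear it, and clicking runs a looping yoyo tween on the flicker mask.
; Debug prints trace both effects; the interact input is empty and a tint tween is unconnected.
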(event OnBeginCursorOver(Mesh)
  (params (TouchedComponent :type Primitive%20Component%20Object%20Reference))
  (Development|PrintText "Me clickearon")
  (CallFunction|Frsesnel true))

(event OnClicked(Mesh)
  (params (TouchedComponent :type Primitive%20Component%20Object%20Reference) (ButtonPressed :type Key%20Structure :default "None"))
  (Development|PrintText "presiono F")
  (CallFunction|Flicker))

(event Custom|Flicker
  (bind _returnvalue (Rendering|Material|GetScalarParameterValue (Variables|/Game/BluePrints/BP_RuntimeMat.BP_RuntimeMat_C|GetruntimeMaterial (Variables|Default|GetBP_RuntimeMat)) (Variables|Default|GetflickerMask) :!class /Script/Engine.MaterialInstanceDynamic))
  (bind _value (|TweenFloat _returnvalue 1.0 1.0 "Linear" 0.0 0.0 0.0 3 0.0 true)
    (:ApplyEasing
      (Rendering|Material|SetScalarParameterValue (Variables|/Game/BluePrints/BP_RuntimeMat.BP_RuntimeMat_C|GetruntimeMaterial (Variables|Default|GetBP_RuntimeMat)) (Variables|Default|GetflickerMask) _value :!class /Script/Engine.MaterialInstanceDynamic)
      (Development|PrintText (Utilities|Text|ToText(Float) _value "HalfToEven") true true "(R=0.000000,G=1.000000,B=0.060579,A=1.000000)" 9.0))))

(event Custom|Frsesnel
  (params (SetActive :type Boolean))
  (bind _bp_runtimemat (Variables|Default|GetBP_RuntimeMat))
  (bind _runtimematerial (Variables|/Game/BluePrints/BP_RuntimeMat.BP_RuntimeMat_C|GetruntimeMaterial _bp_runtimemat))
  (bind _returnvalue (Rendering|Material|GetScalarParameterValue _runtimematerial (Variables|Default|GetfresnelMask) :!class /Script/Engine.MaterialInstanceDynamic))
  (bind _value (|TweenFloat _returnvalue (Math|Conversions|ToFloat(Boolean) SetActive) 0.3 "InOutQuad")
    (:ApplyEasing
      (Rendering|Material|SetScalarParameterValue _runtimematerial (Variables|Default|GetfresnelMask) _value :!class /Script/Engine.MaterialInstanceDynamic)
      (Development|PrintText "Im fresneling")
      (Development|PrintText (Utilities|Text|ToText(Float) _value "HalfToEven")))
    (:OnComplete
      (Development|PrintText "Stoped fresneling"))))

(event Input|EnhancedActionEvents|EnhancedInputActionIA_Intereact
  (params (ActionValue :type Boolean) (ElapsedSeconds :type Float%20%28double-precision%29) (TriggeredSeconds :type Float%20%28double-precision%29) (InputAction :type Input%20Action%20Object%20Reference :default "/Game/BluePrints/IA_Intereact.IA_Intereact")))

(event EventBeginPlay
  (bind _bp_runtimemat (Variables|Default|GetBP_RuntimeMat))
  (bind _runtimematerial (Variables|/Game/BluePrints/BP_RuntimeMat.BP_RuntimeMat_C|GetruntimeMaterial _bp_runtimemat))
  (Default|ApplyRuntimeMaterial _bp_runtimemat (Utilities|Array|MakeArray (Variables|Character|GetMesh)))
  (Rendering|Material|SetScalarParameterValue _runtimematerial (Variables|Default|GetfresnelMask) 0.0 :!class /Script/Engine.MaterialInstanceDynamic)
  (Rendering|Material|SetScalarParameterValue _runtimematerial (Variables|Default|GetflickerMask) 0.0 :!class /Script/Engine.MaterialInstanceDynamic))

(event Input|KeyboardEvents|F
  (params (Key :type Key%20Structure :default "None")))

(fn ConstructionScript)