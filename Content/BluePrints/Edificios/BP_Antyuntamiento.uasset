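; BP_Antyuntamiento is the ant town hall building, serving as resource drop-off and worker spawner, whose destruction loses the game.
; DepositResource forwards a fixed amount of Grass or Clay to the game mode.
; DoMyThingBlue, gated by CheckCanDoMyThing, spawns a BP_HormigaObrera worker at the mushroom mesh's location cached on BeginPlay and passes itself to it.
; OnBuildingDestroy triggers the game mode's loss before running the parent logic.
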(event Custom|DepositResource
  (params (Resource :type ResourceType%20Enum :default "NewEnumerator0"))
  (bind _gamemanager (CallFunction|GetMyGameMode))
  (switch Utilities|FlowControl|Switch|SwitchonResourceType Resource
    (:NewEnumerator0
      (Default|UpdateGrass _gamemanager 100))
    (:NewEnumerator1
      (Default|UpdateClay _gamemanager 100))))

(event EventBeginPlay
  (|CallParentFunction)
  (Variables|Default|SetSpawn%20Transform (Math|Transform|MakeTransform (Transformation|GetWorldLocation (Variables|Default|GetSM_DeathCapBAdultVariantC)) "0, 0, 0" "1.000000,1.000000,1.000000")))

(event EventOnBuildingDestroy
  (bind _gamemanager (CallFunction|GetMyGameMode))
  (Default|OnGameLoss _gamemanager)
  (|CallParentFunction))

(fn ConstructionScript)

(fn DoMyThingBlue
  (bind _can (CallFunction|CheckCanDoMyThing))
  (if _can
    (bind _returnvalue (Game|SpawnActorfromClass "/Game/BluePrints/BP_HormigaObrera.BP_HormigaObrera_C" (Variables|Default|GetSpawn%20Transform) "AdjustIfPossibleButAlwaysSpawn" "MultiplyWithRoot" 0 0))
    (Default|RecibirAyuntamiento _returnvalue self)))