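; BP_BlackAntyuntamiento is the enemy black ant town hall building, whose destruction triggers the game win.
; A Delay on Tick paces spawns of black warrior ants at a foxglove mesh's location, each sent toward the first BP_Antyuntamiento found at BeginPlay.
; Each spawn shortens the delay, and spawning stops once it drops below a fixed threshold.
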(event EventBeginPlay
  (|CallParentFunction)
  (Variables|Default|SetSpawnTransform (Math|Transform|MakeTransform (Transformation|GetWorldLocation (Variables|Default|GetSM_FoxgloveBVariantB)) "0, 0, 0" "1.000000,1.000000,1.000000"))
  (bind _outactors (Actor|GetAllActorsOfClass "/Game/BluePrints/Edificios/BP_Antyuntamiento.BP_Antyuntamiento_C"))
  (Variables|Default|SetAntyuntamiento%20Rojo (Utilities|Array|Get(acopy) _outactors)))

(event EventTick
  (params (DeltaSeconds :type Float%20%28single-precision%29))
  (Utilities|FlowControl|Delay (Variables|Default|GetTime%20to%20Spawn%20))
  (if (>= (Variables|Default|GetTime%20to%20Spawn%20) 5.0)
    (Variables|Default|SetTime%20to%20Spawn%20 (- (Variables|Default|GetTime%20to%20Spawn%20) 0.5))
    (bind _out_ant (CallFunction|SpawnBalckAnt))
    (Default|MovetoActor _out_ant (Variables|Default|GetAntyuntamiento%20Rojo))))

(event EventOnBuildingDestroy
  (bind _gamemanager (CallFunction|GetMyGameMode))
  (Default|OnGameWon _gamemanager)
  (|CallParentFunction))

(fn ConstructionScript
  (|CallParentFunction))

(fn SpawnBalckAnt
  (bind _returnvalue (Game|SpawnActorfromClass "/Game/BluePrints/BP_HormigaGuerreraNegra.BP_HormigaGuerreraNegra_C" (Variables|Default|GetSpawnTransform) "AlwaysSpawn" "MultiplyWithRoot" 0 0))
  (return _returnvalue))