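; BP_GrassDeposit is a grass deposit actor among the building Blueprints.
; On BeginPlay it passes three static mesh components to BPRuntimeMat to apply a runtime material, then calls DoMyThingBlue, whose body is not defined here.
; Its construction script only runs the parent's, and its overlap and tick events are disabled.
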(event EventBeginPlay
  (Default|ApplyRuntimeMaterial (Variables|Default|GetBP_RuntimeMat) (Utilities|Array|MakeArray (Variables|Default|GetStaticMesh2) (Variables|Default|GetStaticMesh) (Variables|Default|GetStaticMesh4)))
  (CallFunction|DoMyThingBlue))

(event Collision|EventActorBeginOverlap
  (params (OtherActor :type Actor%20Object%20Reference))
  (|CallParentFunction OtherActor) ; This node is disabled and will not be called.\nDrag off pins to build functionality.
)

(event EventTick
  (params (DeltaSeconds :type Float%20%28single-precision%29))
  (|CallParentFunction DeltaSeconds) ; This node is disabled and will not be called.\nDrag off pins to build functionality.
)

(fn ConstructionScript
  (|CallParentFunction))