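; RTS building actor that can be hovered, click-selected and destroyed, with animated material feedback.
; Box collider clicks toggle its entry in BP_RTSGameManager's selected list, and hovering shows a Fresnel highlight that persists while selected.
; BPRuntimeMat supplies the runtime material, whose Fresnel, flicker and dither parameters are driven by float tweens from their current values.
; Destruction tweens the dither mask to zero and plays a sound at the building's location.
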(event OnClicked(BoxCollider)
  (params (TouchedComponent :type Primitive%20Component%20Object%20Reference) (ButtonPressed :type Key%20Structure :default "None"))
  (CallFunction|ToggleSelect))

(event OnBeginCursorOver(BoxCollider)
  (params (TouchedComponent :type Primitive%20Component%20Object%20Reference))
  (CallFunction|Fresnel true))

(event OnEndCursorOver(BoxCollider)
  (params (TouchedComponent :type Primitive%20Component%20Object%20Reference))
  (bind _asbp_rtsgame_manager (Utilities|Casting|CastToBP_RTSGameManager (Game|GetGameMode)))
  (bind _itexists (Default|ItemExistonSelectedList _asbp_rtsgame_manager self))
  (if (not _itexists)
    (CallFunction|Fresnel false)))

(event Custom|Flicker
  (|FlickerCollapsed))

(event Custom|Fresnel
  (params (SetActive :type Boolean))
  (|FresnelColapsed SetActive))

(event Custom|ToggleSelect
  (|ToggleSelectCollapsed))

(event Custom|Deselect
  (CallFunction|Fresnel false))

(event Custom|OnBuildingDestroy
  (CallFunction|Dither)
  (Audio|PlaySoundatLocation (Variables|Default|GetDestroySoundEfect) (Transformation|GetWorldLocation (Variables|Default|GetDefaultSceneRoot)) "0, 0, 0" 1.0 1.0 0.0 0 0 0 0))

(event Custom|Dither
  (|CollapsedDither))

(event EventBeginPlay
  (|BeginCollapsed))

(fn ConstructionScript)

(fn DoMyThingBlue
  (Development|PrintText (Utilities|Text|ToText(String) (Utilities|GetObjectName self))))

(fn GetMyGameMode
  (bind _asbp_rtsgame_manager (Utilities|Casting|CastToBP_RTSGameManager (Game|GetGameMode)))
  (return _asbp_rtsgame_manager))