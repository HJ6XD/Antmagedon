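; BP_BlackFarm is a building Blueprint for a farm structure that affects the game's grass and clay resources.
; On BeginPlay it applies a runtime material to its farm and plant meshes, then zeroes the fresnel and flicker masks.
; When destroyed, it passes a fixed positive amount to the game mode's grass and clay updates before running the parent's destroy logic.
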(event EventBeginPlay
  (bind _bp_runtimemat (Variables|Default|GetBP_RuntimeMat))
  (bind _runtimematerial (Variables|/Game/BluePrints/BP_RuntimeMat.BP_RuntimeMat_C|GetruntimeMaterial _bp_runtimemat))
  (Default|ApplyRuntimeMaterial _bp_runtimemat (Utilities|Array|MakeArray (Variables|Default|GetStaticMesh) (Variables|Default|GetSM_DeathCapBAdultVariantC) (Variables|Default|GetSM_MixedGrassLumpLargeB)))
  (Rendering|Material|SetScalarParameterValue _runtimematerial (Variables|Default|GetfresnelMask) 0.0 :!class /Script/Engine.MaterialInstanceDynamic)
  (Rendering|Material|SetScalarParameterValue _runtimematerial (Variables|Default|GetFlickerMask) 0.0 :!class /Script/Engine.MaterialInstanceDynamic))

(event EventOnBuildingDestroy
  (bind _gamemanager (CallFunction|GetMyGameMode))
  (Default|UpdateGrass _gamemanager 1000)
  (Default|UpdateClay _gamemanager 1000)
  (|CallParentFunction))

(event EventTick
  (params (DeltaSeconds :type Float%20%28single-precision%29)))

(fn ConstructionScript
  (|CallParentFunction))