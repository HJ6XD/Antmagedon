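; BP_RTSGameManager is the central manager for an ant RTS, holding selection, grass and clay resources, army size and win/loss handling.
; On BeginPlay it shows the cursor and creates the WBP_PlayerUI, which its update functions refresh as values change.
; Selection holds one class at a time, deselecting ants and buildings when cleared and toggling building panels.
; It also tracks warrior ants and a buff count, and pauses on game end.
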(event Custom|RemoveFromSelectedList
  (params (actorToRemove :type Actor%20Object%20Reference))
  (Utilities|Casting|CastToBP_Edificio actorToRemove
    (:then
      (Default|SetDMTPanelVisibility (Variables|Default|GetGameUI) false))
    (:CastFailed
      _))
  (Utilities|Array|RemoveItem (Variables|Default|GetselectedList) actorToRemove))

(event Custom|AddToSelectedList
  (params (actorToAdd :type Actor%20Object%20Reference))
  (bind _selectedlist (Variables|Default|GetselectedList))
  (if (> (Utilities|Array|Length _selectedlist) 0)
    (if (== (Utilities|GetClass actorToAdd) (Utilities|GetClass (Utilities|Array|Get(acopy) _selectedlist)))
      _
      (else
        (CallFunction|ClearSelectedList))))
  (Utilities|Array|Add _selectedlist actorToAdd)
  (bind _output_get (Variables|Default|SetLastSelected actorToAdd))
  (Utilities|Casting|CastToBP_Edificio _output_get)
  (Default|DisplayBuildingInfo (Variables|Default|GetGameUI)))

(event Custom|AddTo%20GuerrerasList
  (params (Guerrera%20To%20Add :type BP%20Hormiga%20Guerrera%20Roja%20Object%20Reference))
  (Utilities|Array|Add (Variables|Default|GetGuerreasList) Guerrera%20To%20Add))

(event Custom|AddTotalBuffCount
  (bind _result (Math|Integer|IncrementInt (Variables|Default|GetTotalBuffCount))
    (:%20%20
      (Variables|Default|SetTotalBuffCount _result))))

(event Custom|ClearSelectedList
  (bind _selectedlist (Variables|Default|GetselectedList))
  (for _array_element _selectedlist
    (bind _asbp_hormiga_t (Utilities|Casting|CastToBP_HormigaT _array_element)
      (:then
        (Default|Deselect _asbp_hormiga_t))
      (:CastFailed
        (bind _asbp_edificio (Utilities|Casting|CastToBP_Edificio _array_element))
        (Default|Deselect _asbp_edificio)
        (Default|SetDMTPanelVisibility (Variables|Default|GetGameUI) false))))
  (Utilities|Array|Clear _selectedlist))

(event Custom|OnGameLoss
  (Game|SetGamePaused true)
  (Default|ActivateGameLossScreen (Variables|Default|GetGameUI)))

(event Custom|OnGameWon
  (Game|SetGamePaused true)
  (Default|ActivateGameWonScreen (Variables|Default|GetGameUI)))

(event EventBeginPlay
  (Variables|/Script/Engine.PlayerController|SetbShowMouseCursor (Game|GetPlayerController 0) true)
  (bind _returnvalue (UserInterface|CreateWidget "/Game/Widgets/WBP_PlayerUI.WBP_PlayerUI_C"))
  (bind _output_get (Variables|Default|SetGameUI _returnvalue))
  (UserInterface|Viewport|AddtoViewport _output_get 0)
  (Default|UpdateCurAS (Variables|Default|GetGameUI) (Variables|Default|GetcurArmySize))
  (Default|UpdateCurClayValue (Variables|Default|GetGameUI) (Variables|Default|GetClayValue))
  (Default|UpdateCurGrassValue (Variables|Default|GetGameUI) (Variables|Default|GetGrassValue))
  (Default|UpdateMaxAS (Variables|Default|GetGameUI) (Variables|Default|GetmaxArmySize)))

(event EventTick
  (params (DeltaSeconds :type Float%20%28single-precision%29)))

(fn ConstructionScript)

(fn ItemExistonSelectedList
  (params (ActorToCheck :type Actor%20Object%20Reference))
  (return (Utilities|Array|ContainsItem (Variables|Default|GetselectedList) ActorToCheck)))

(fn UpdateGrass
  (params (GrassPlus :type Integer))
  (bind _output_get (Variables|Default|SetGrassValue (+ (Variables|Default|GetGrassValue) GrassPlus)))
  (Default|UpdateCurGrassValue (Variables|Default|GetGameUI) _output_get))

(fn UpdateClay
  (params (ClayPlus :type Integer))
  (bind _output_get (Variables|Default|SetClayValue (+ (Variables|Default|GetClayValue) ClayPlus)))
  (Default|UpdateCurClayValue (Variables|Default|GetGameUI) _output_get))

(fn UpdateMaxArmySize
  (params (MASPlus :type Integer))
  (bind _output_get (Variables|Default|SetmaxArmySize (+ (Variables|Default|GetmaxArmySize) MASPlus)))
  (Default|UpdateMaxAS (Variables|Default|GetGameUI) _output_get))

(fn UpdateCurArmySize
  (params (CASPlus :type Integer))
  (bind _output_get (Variables|Default|SetcurArmySize (+ (Variables|Default|GetcurArmySize) CASPlus)))
  (Default|UpdateCurAS (Variables|Default|GetGameUI) _output_get))