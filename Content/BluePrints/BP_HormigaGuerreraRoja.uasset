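; Red warrior ant unit for an RTS, a child Blueprint that attacks black ant warriors and buildings.
; On BeginPlay it sets its health and reports its size to the RTS game manager's army count.
; Its RepeatingAction override runs the parent logic, then attacks the first matching target in OutActors.
; A Buff event scales max health and damage by DamageBuff, rounding up and refilling health.
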(event Custom|Buff
  (bind _damagebuff (Variables|Default|GetDamageBuff))
  (bind _output_get (Variables|Default|SetmaxHP (Math|Float|Ceil (* _damagebuff (Variables|Default|GetmaxHP)))))
  (Variables|Default|SetcurHP _output_get)
  (Variables|Default|SetDamage (Math|Float|Ceil (* _damagebuff (Variables|Default|GetDamage)))))

(event EventBeginPlay
  (|CallParentFunction)
  (bind _output_get (Variables|Default|SetmaxHP 150))
  (Variables|Default|SetcurHP _output_get)
  (bind _asbp_rtsgame_manager (Utilities|Casting|CastToBP_RTSGameManager (Game|GetGameMode)))
  (Default|UpdateCurArmySize _asbp_rtsgame_manager (Variables|Default|GetSize)))

(event Collision|EventActorBeginOverlap
  (params (OtherActor :type Actor%20Object%20Reference))
  (|CallParentFunction OtherActor) ; This node is disabled and will not be called.\nDrag off pins to build functionality.
)

(event EventTick
  (params (DeltaSeconds :type Float%20%28single-precision%29))
  (|CallParentFunction DeltaSeconds) ; This node is disabled and will not be called.\nDrag off pins to build functionality.
)

(fn ConstructionScript
  (|CallParentFunction))

(fn ArriveAction
  (|CallParentFunction))

(fn RepeatingAction
  (|CallParentFunction)
  (for _array_element (Variables|Default|GetOut%20Actors)
    (bind _asbp_hormiga_guerrera_negra (Utilities|Casting|CastToBP_HormigaGuerreraNegra _array_element)
      (:then
        (Variables|Default|SetTargetActorToAtack _asbp_hormiga_guerrera_negra))
      (:CastFailed
        (bind _asbp_black_ant_building (Utilities|Casting|CastToBP_BlackAntBuilding _array_element))
        (Variables|Default|SetTargetActorToAtack _asbp_black_ant_building)))
    (CallFunction|Atack)
    (return false))
  (return false))