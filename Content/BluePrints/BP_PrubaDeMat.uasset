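; Test actor for runtime material effects, using a BPRuntimeMat component that applies a runtime material to its mesh.
; Fresnel and flicker masks start at zero; clicking the mesh tweens the Fresnel mask on, with debug prints.
; A Flicker event tweens its mask but is not called here.
; The F key starts a looping tint tween, which writes only on yoyo to a parameter named "None".
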(event OnClicked(Mesh)
  (params (TouchedComponent :type Primitive%20Component%20Object%20Reference) (ButtonPressed :type Key%20Structure :default "None"))
  (Development|PrintText "Me clickearon")
  (CallFunction|Frsesnel true))

(event Custom|Flicker
  (bind _returnvalue (Rendering|Material|GetScalarParameterValue (Variables|/Game/BluePrints/BP_RuntimeMat.BP_RuntimeMat_C|GetruntimeMaterial (Variables|Default|GetBP_RuntimeMat)) (Variables|Default|GetflickerMask) :!class /Script/Engine.MaterialInstanceDynamic))
  (bind _value (|TweenFloat _returnvalue 1.0 1.0 "InOutQuad" 0.0 0.0 0.0 3 0.0 true 0.5)
    (:ApplyEasing
      (Rendering|Material|SetScalarParameterValue (Variables|/Game/BluePrints/BP_RuntimeMat.BP_RuntimeMat_C|GetruntimeMaterial (Variables|Default|GetBP_RuntimeMat)) (Variables|Default|GetflickerMask) _value :!class /Script/Engine.MaterialInstanceDynamic))))

(event Custom|Frsesnel
  (params (SetActive :type Boolean))
  (bind _bp_runtimemat (Variables|Default|GetBP_RuntimeMat))
  (bind _runtimematerial (Variables|/Game/BluePrints/BP_RuntimeMat.BP_RuntimeMat_C|GetruntimeMaterial _bp_runtimemat))
  (bind _returnvalue (Rendering|Material|GetScalarParameterValue _runtimematerial (Variables|Default|GetfresnelMask) :!class /Script/Engine.MaterialInstanceDynamic))
  (bind _value (|TweenFloat _returnvalue (Math|Conversions|ToFloat(Boolean) SetActive) 0.3 "InOutQuad")
    (:ApplyEasing
      (Rendering|Material|SetScalarParameterValue _runtimematerial (Variables|Default|GetfresnelMask) _value :!class /Script/Engine.MaterialInstanceDynamic)
      (Development|PrintText "Im fresneling")
      (Development|PrintText (Utilities|Text|ToText(Float) _value "HalfToEven")))
    (:OnComplete
      (Development|PrintText "Stoped fresneling"))))

(event EventBeginPlay
  (bind _bp_runtimemat (Variables|Default|GetBP_RuntimeMat))
  (bind _runtimematerial (Variables|/Game/BluePrints/BP_RuntimeMat.BP_RuntimeMat_C|GetruntimeMaterial _bp_runtimemat))
  (Default|ApplyRuntimeMaterial _bp_runtimemat (Utilities|Array|MakeArray (Variables|Character|GetMesh)))
  (Rendering|Material|SetScalarParameterValue _runtimematerial (Variables|Default|GetfresnelMask) 0.0 :!class /Script/Engine.MaterialInstanceDynamic)
  (Rendering|Material|SetScalarParameterValue _runtimematerial (Variables|Default|GetflickerMask) 0.0 :!class /Script/Engine.MaterialInstanceDynamic))

(event Input|KeyboardEvents|F
  (params (Key :type Key%20Structure :default "None"))
  (bind _bp_runtimemat (Variables|Default|GetBP_RuntimeMat))
  (bind _runtimematerial (Variables|/Game/BluePrints/BP_RuntimeMat.BP_RuntimeMat_C|GetruntimeMaterial _bp_runtimemat))
  (:Pressed
    (bind _returnvalue (Rendering|Material|GetVectorParameterValue _runtimematerial (Variables|Default|GettintParameter) :!class /Script/Engine.MaterialInstanceDynamic))
    (bind _value (|TweenVector (Math|Conversions|ToVector(LinearColor) _returnvalue) (Math|Conversions|ToVector(LinearColor) (Math|Conversions|ToLinearColor(Color) (Variables|Default|GetTintColor))) 1.0 "InOutQuad" 0.0 0.0 0.0 3 0.0 true)
      (:OnYoyo
        (Rendering|Material|SetVectorParameterValue _runtimematerial "None" (Math|Conversions|ToLinearColor(Vector) _value) :!class /Script/Engine.MaterialInstanceDynamic)))))

(fn ConstructionScript)